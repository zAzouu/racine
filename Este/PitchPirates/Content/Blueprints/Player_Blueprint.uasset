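; Player character Blueprint that handles walking and sprinting from player input.
; MoveX and MoveY axes add movement input along the right and forward vectors of the control rotation's yaw, so movement follows the controller's horizontal heading.
; The Sprint action switches the movement component's max walk speed to SprintSpeed while held and back to WalkSpeed on release.
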(event Input|ActionEvents|InputActionSprint
  (params (Key :type Key%20Structure :default "AnyKey"))
  (bind _charactermovement (Variables|Character|GetCharacterMovement))
  ;[1 1 1] Sprint
  (:Pressed
    (Variables|/Script/Engine.CharacterMovementComponent|SetMaxWalkSpeed _charactermovement (Variables|Default|GetSprintSpeed)))
  (:Released
    (Variables|/Script/Engine.CharacterMovementComponent|SetMaxWalkSpeed _charactermovement (Variables|Default|GetWalkSpeed))))

(event Input|AxisEvents|InputAxisMoveX
  (params (AxisValue :type Float%20%28single-precision%29))
  ;[1 1 1] Move
  (Pawn|Input|AddMovementInput (Math|Vector|GetRightVector (Math|Rotator|MakeRotator 0.0 0.0 (.Yaw (Math|Rotator|BreakRotator (Pawn|GetControlRotation :!class /Script/Engine.Pawn))))) AxisValue false))

(event Input|AxisEvents|InputAxisMoveY
  (params (AxisValue :type Float%20%28single-precision%29))
  ;[1 1 1] Move
  (Pawn|Input|AddMovementInput (Math|Vector|GetForwardVector (Math|Rotator|MakeRotator 0.0 0.0 (.Yaw (Math|Rotator|BreakRotator (Pawn|GetControlRotation :!class /Script/Engine.Pawn))))) AxisValue false))

(fn ConstructionScript)